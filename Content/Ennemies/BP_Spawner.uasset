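; Enemy spawner Blueprint that offers one function each to spawn basic, tank, medium and flying enemy AI.
; Each function spawns its pawn class at the supplied location plus SpawnOffset, with random jitter on X, ignoring collision.
; The flying spawn then teleports the new enemy by its own MaxHeight offset.
; The event graph and construction script are empty, so the Blueprint does not trigger any spawns itself.
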(event `self.ReceiveBeginPlay`)

(event `self.ReceiveTick`
  (params (DeltaSeconds :type "Float (single-precision)")))

(fn `Spawn Flying Ennemy`
  (params (Location :type "Vector Structure"))
  (bind _returnvalue (`AIBlueprintHelperLibrary.SpawnAIFromClass` "/Game/Ennemies/BP_FlyingEnemy.BP_FlyingEnemy_C" null (+ Location (`KismetMathLibrary.MakeVector` (+ (.x (`self.SpawnOffset`)) (`KismetMathLibrary.RandomFloatInRange` 0.0 10.0)) (.y (`self.SpawnOffset`)) (.z (`self.SpawnOffset`)))) (struct) true null))
  (bind _asbp_flying_enemy (cast `/Game/Ennemies/BP_FlyingEnemy` _returnvalue))
  (`self.K2_SetActorLocation` _asbp_flying_enemy (+ (`self.K2_GetActorLocation` _asbp_flying_enemy) (`/Game/Ennemies/BP_FlyingEnemy.Max Height` _asbp_flying_enemy)) false true))

(fn `Spawn Medium Ennemy`
  (params (Location :type "Vector Structure"))
  (`AIBlueprintHelperLibrary.SpawnAIFromClass` "/Game/Ennemies/BP_Medium_EnnemyChild.BP_Medium_EnnemyChild_C" null (+ Location (`KismetMathLibrary.MakeVector` (+ (.x (`self.SpawnOffset`)) (`KismetMathLibrary.RandomFloatInRange` 0.0 10.0)) (.y (`self.SpawnOffset`)) (.z (`self.SpawnOffset`)))) (struct) true null))

(fn `Spawn Tank Ennemy`
  (params (Location :type "Vector Structure"))
  (`AIBlueprintHelperLibrary.SpawnAIFromClass` "/Game/Ennemies/BP_TankEnemy.BP_TankEnemy_C" null (+ Location (`KismetMathLibrary.MakeVector` (+ (.x (`self.SpawnOffset`)) (`KismetMathLibrary.RandomFloatInRange` 0.0 10.0)) (.y (`self.SpawnOffset`)) (.z (`self.SpawnOffset`)))) (struct) true null))

(fn `SpawnBasicEnnemy`
  (params (Location :type "Vector Structure"))
  (`AIBlueprintHelperLibrary.SpawnAIFromClass` "/Game/Ennemies/BP_BasicEnemy.BP_BasicEnemy_C" null (+ Location (`KismetMathLibrary.MakeVector` (+ (.x (`self.SpawnOffset`)) (`KismetMathLibrary.RandomFloatInRange` 0.0 10.0)) (.y (`self.SpawnOffset`)) (.z (`self.SpawnOffset`)))) (struct) true null))

(fn `UserConstructionScript`)