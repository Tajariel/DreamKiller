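; Medium enemy that chases the player and damages them on contact.
; Every Tick it issues AIMoveTo toward the player character, and Hit calls TakeDamage on BP_FirstPersonCharacter with the enemy's rotation.
; Radial damage lowers EnnemyPV and destroys the actor at zero or below.
; TimedExplosion applies player-credited radial damage with a debug sphere and particle burst, but nothing here calls it.
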(event `self.ReceiveTick`
  (params (DeltaSeconds :type "Float (single-precision)"))
  ;[1 1 1] Make Ennemy follow Player
  (`|AIMoveTo` self (0.0 0.0 0.0) (`GameplayStatics.GetPlayerCharacter` 0)))

(event `self.ReceiveHit`
  (params (MyComp :type "PrimitiveComponent Object Reference") (Other :type "Actor Object Reference") (OtherComp :type "PrimitiveComponent Object Reference") (bSelfMoved :type Boolean) (HitLocation :type "Vector Structure") (HitNormal :type "Vector Structure") (NormalImpulse :type "Vector Structure") (Hit :type "HitResult Structure (by ref)"))
  ;[1 1 1] When Hit Inflict damage to player
  (bind _asbp_first_person_character (cast `/Game/FirstPerson/Blueprints/BP_FirstPersonCharacter` Other))
  (`/Game/FirstPerson/Blueprints/BP_FirstPersonCharacter.TakeDamage` _asbp_first_person_character (`self.K2_GetActorRotation`)))

(event `self.ReceiveRadialDamage`
  (params (DamageReceived :type "Float (single-precision)") (DamageType :type "DamageType Object Reference") (Origin :type "Vector Structure") (HitInfo :type "HitResult Structure (by ref)") (InstigatedBy :type "Controller Object Reference") (DamageCauser :type "Actor Object Reference"))
  (bind _output_get (set `self.EnnemyPV` (`KismetMathLibrary.FTrunc` (- (`self.EnnemyPV`) DamageReceived))))
  (if (<= _output_get 0)
    (`self.K2_DestroyActor`)))

(fn `TimedExplosion`
  (bind _returnvalue (`self.K2_GetActorLocation`))
  (`KismetSystemLibrary.DrawDebugSphere` _returnvalue 300.0 12 (struct :`R` 1.0 :`G` 1.0 :`B` 1.0 :`A` 1.0) 3.0)
  (`GameplayStatics.ApplyRadialDamage` :`BaseDamage` 50.0 :`Origin` _returnvalue :`DamageRadius` 300.0 :`DamageCauser` (`GameplayStatics.GetPlayerCharacter` 0) :`InstigatedByController` (`GameplayStatics.GetPlayerController` 0) :`bDoFullDamage` true)
  (`GameplayStatics.SpawnEmitterAtLocation` "/Game/StarterContent/Particles/P_Explosion.P_Explosion" _returnvalue (struct) (5.0 5.0 5.0)))

(fn `UserConstructionScript`)