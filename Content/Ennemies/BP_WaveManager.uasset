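; BP_WaveManager is a trigger actor that runs one enemy wave, started when an actor overlaps it.
; BeginPlay fills a type-ID array from the basic, medium, tank and flying enemy counts.
; Once triggered, Tick uses a Delay to pace spawns, drawing random entries without replacement and sending each to a random spawner.
; EnnemyKilled counts down the remaining enemies, then destroys the spawners and the manager when none remain.
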(event `self.ReceiveBeginPlay`
  (for _ (range 1 (+ (`self.BasicEnnemyNumber`) 1))
    (`KismetArrayLibrary.Array_Add` (`self.WaveContent`)))
  (for _ (range 1 (+ (`self.MediumEnnemyNumber`) 1))
    (`KismetArrayLibrary.Array_Add` (`self.WaveContent`) 1))
  (for _ (range 1 (+ (`self.TankEnnemyNumber`) 1))
    (`KismetArrayLibrary.Array_Add` (`self.WaveContent`) 2))
  (for _ (range 1 (+ (`self.FlyingEnnemyNumber`) 1))
    (`KismetArrayLibrary.Array_Add` (`self.WaveContent`) 3))
  (set `self.LeftToKill` (`KismetArrayLibrary.Array_Length` (`self.WaveContent`))))

(event `self.ReceiveActorBeginOverlap`
  (params (OtherActor :type "Actor Object Reference"))
  (set `self.IsOn` true))

(event `self.ReceiveTick`
  (params (DeltaSeconds :type "Float (single-precision)"))
  (bind _spawners (`self.Spawners`))
  (if (`self.IsOn`)
    (if (not (== (`KismetArrayLibrary.Array_Length` (`self.WaveContent`)) 0))
      (`KismetSystemLibrary.Delay` 1.0)
      (`self.SpawnEnmyFromSpwnr` (`|GetArrayItem` _spawners (`KismetMathLibrary.RandomInteger` (`KismetArrayLibrary.Array_Length` _spawners))) (`KismetMathLibrary.RandomInteger` (`KismetArrayLibrary.Array_Length` (`self.WaveContent`)))))))

(event `EnnemyKilled`
  (bind _output_get (set `self.LeftToKill` (- (`self.LeftToKill`) 1)))
  (if (<= _output_get 0)
    (for _array_element (`self.Spawners`)
      (`self.K2_DestroyActor` _array_element))
    (`self.K2_DestroyActor`)))

(fn `SpawnEnmyFromSpwnr`
  (params (Spawner :type "/Game/Ennemies/BP_Spawner Object Reference") (EnnemyType :type Integer))
  (bind _returnvalue (`self.K2_GetActorLocation` Spawner))
  (bind _wavecontent (`self.WaveContent`))
  (switch `int` (`|GetArrayItem` (`self.WaveContent`) EnnemyType)
    (:`0`
      (`/Game/Ennemies/BP_Spawner.SpawnBasicEnnemy` Spawner _returnvalue null))
    (:`1`
      (`/Game/Ennemies/BP_Spawner.Spawn Medium Ennemy` Spawner _returnvalue))
    (:`2`
      (`/Game/Ennemies/BP_Spawner.Spawn Tank Ennemy` Spawner _returnvalue))
    (:`3`
      (`/Game/Ennemies/BP_Spawner.Spawn Flying Ennemy` Spawner _returnvalue)))
  (`KismetArrayLibrary.Array_Remove` _wavecontent EnnemyType)
  (`KismetSystemLibrary.PrintString` (`KismetStringLibrary.Conv_IntToString` (`KismetArrayLibrary.Array_Length` _wavecontent))))

(fn `UserConstructionScript`)