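; Medium enemy child Blueprint that sets its health (EnnemyPV) on BeginPlay and turns to face the player.
; Each Tick, while the blackboard's TargetActor is valid, it snaps its rotation toward player character 0 rather than that stored actor.
; FireAtPlayer only checks IsFiring and performs no action, and the construction script just calls the parent's.
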(event `self.ReceiveBeginPlay`
  (set `self.EnnemyPV` 30))

(event `self.ReceiveTick`
  (params (DeltaSeconds :type "Float (single-precision)"))
  (`/Engine/EditorBlueprintResources/StandardMacros.IsValid` (`BlackboardComponent.GetValueAsObject` (`AIBlueprintHelperLibrary.GetBlackboard` null) "TargetActor")
    (:`Is Valid`
      (`self.K2_SetActorRotation` (`KismetMathLibrary.FindLookAtRotation` (`self.K2_GetActorLocation`) (`self.K2_GetActorLocation` (`GameplayStatics.GetPlayerCharacter` 0)))))))

(fn `FireAtPlayer`
  (if (`self.IsFiring`)
    _))

(fn `UserConstructionScript`
  (`parent.UserConstructionScript`))